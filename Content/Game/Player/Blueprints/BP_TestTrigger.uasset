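; BP_TestTrigger is a test trigger volume that starts a battle when the player character BP_Gustav enters its box.
; On overlap it switches Gustav's state machine into combat mode, then spawns a BP_BattleManager at the world origin.
; If the manager spawns validly it starts the battle and disables the box's collision, so the trigger fires only once.
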(event OnComponentBeginOverlap(Box)
  (params (OverlappedComponent :type Primitive%20Component%20Object%20Reference) (OtherActor :type Actor%20Object%20Reference) (OtherComp :type Primitive%20Component%20Object%20Reference) (OtherBodyIndex :type Integer) (bFromSweep :type Boolean) (SweepResult :type Hit%20Result%20Structure%20%28by%20ref%29))
  (bind _asbp_gustav (Utilities|Casting|CastToBP_Gustav OtherActor))
  (Class|PlayerFSM|EnterCombatMode (Variables|/Script/ClairObscur.PlayerBase|Getfsm _asbp_gustav))
  (bind _returnvalue (Game|SpawnActorfromClass "/Game/Game/BattleSystem/BP_BattleManager.BP_BattleManager_C" (Math|Transform|MakeTransform (Math|Vector|MakeVector 0.0 0.0 0.0) "0, 0, 0" "1.000000,1.000000,1.000000") "Undefined" "MultiplyWithRoot" 0 0))
  (bind _output_get (Variables|Default|SetBM _returnvalue))
  (Utilities|IsValid _output_get
    (:Is%20Valid
      (Class|BattleManager|StartBattle (Variables|Default|GetBm))
      (Collision|SetCollisionEnabled (Variables|Default|GetBox) "NoCollision"))))

(event EventBeginPlay)

(event Collision|EventActorBeginOverlap
  (params (OtherActor :type Actor%20Object%20Reference)))

(event EventTick
  (params (DeltaSeconds :type Float%20%28single-precision%29)))

(fn ConstructionScript)