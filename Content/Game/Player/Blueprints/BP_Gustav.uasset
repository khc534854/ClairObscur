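; BP_Gustav is the player Blueprint for Gustav, set up as a test bed for combat skills and animation switching.
; On BeginPlay it puts its Fsm component into combat and caches a Testenemy actor, which TestSkill targets by location when executing the first skill.
; Custom events swap the mesh between combat and default Anim Blueprints.
; Key 2 restores the default, while the local calls to the combat swap and skill test are disconnected.
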(event Custom|TestSkill
  (Variables|Default|GetTestENemy
    (:then
      (Development|PrintString "Hello")
      (Class|PlayerFSM|ExecuteSkill (Variables|Default|Getfsm) (Transformation|GetActorLocation (Variables|Default|GetTestENemy))))
    (:else)))

(event Custom|changecombat
  (Components|SkeletalMesh|SetAnimInstanceClass (Variables|Character|GetMesh) "/Game/Game/Player/ABP/ABP_Gustav_Combat.ABP_Gustav_Combat_C"))

(event Custom|backabp
  (Components|SkeletalMesh|SetAnimInstanceClass (Variables|Character|GetMesh) "/Game/Game/Player/ABP/ABP_Gustav.ABP_Gustav_C"))

(event EventBeginPlay
  (Variables|/Script/ClairObscur.PlayerFSM|SetbIsInCombat (Variables|Default|Getfsm) true)
  (bind _returnvalue (Actor|GetActorOfClass "/Game/Game/Player/Blueprints/testenemy.testenemy_C"))
  (Variables|Default|SetTestENemy _returnvalue))

(event Input|KeyboardEvents|2
  (params (Key :type Key%20Structure :default "None"))
  (:Pressed
    (CallFunction|Backabp)))

(fn ConstructionScript)