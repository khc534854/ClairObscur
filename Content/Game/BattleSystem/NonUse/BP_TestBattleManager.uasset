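; BP_TestBattleManager is a test battle manager that sets up a timing-based combat prototype.
; On BeginPlay it gathers test players and enemies into two parties, shows the WBP_TESTTiming widget and enables player input.
; Unconnected graph chains hold a timing-window check with printed feedback, plus delayed first-skill montage playback for each party's first member, so none of that combat logic runs.
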(event EventBeginPlay
  (bind _outactors (Actor|GetAllActorsOfClass "/Game/Game/BattleSystem/NonUse/BP_TestPlayer.BP_TestPlayer_C"))
  (Variables|Default|SetPlayerParty _outactors)
  (bind _outactors_2 (Actor|GetAllActorsOfClass "/Game/Game/BattleSystem/NonUse/BP_TestEnemy.BP_TestEnemy_C"))
  (Variables|Default|SetEnemyParty _outactors_2)
  (bind _returnvalue (UserInterface|CreateWidget "/Game/Game/BattleSystem/TestUI/WBP_TESTTiming.WBP_TESTTiming_C"))
  (bind _output_get (Variables|Default|SetTimingWidget _returnvalue))
  (UserInterface|Viewport|AddtoViewport _output_get 0)
  (Input|EnableInput (Game|GetPlayerController 0)))

(event Input|KeyboardEvents|E
  (params (Key :type Key%20Structure :default "None")))

(event Input|KeyboardEvents|SpaceBar
  (params (Key :type Key%20Structure :default "None")))

(event Input|KeyboardEvents|Q
  (params (Key :type Key%20Structure :default "None")))

(fn ConstructionScript)