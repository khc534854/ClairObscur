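; Box trigger that starts a battle on overlap and swaps the Explore music it plays at BeginPlay for Battle music.
; The overlap disables the box, puts every PlayerBase FSM into combat mode and calls StartBattle on the first BP_BattleManager found.
; It then rescales and re-initializes animation on the first BP_Enemy and blends the camera to the manager.
; A level sequence intro exists but is disconnected.
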(event OnComponentBeginOverlap(Box)
  (params (OverlappedComponent :type Primitive%20Component%20Object%20Reference) (OtherActor :type Actor%20Object%20Reference) (OtherComp :type Primitive%20Component%20Object%20Reference) (OtherBodyIndex :type Integer) (bFromSweep :type Boolean) (SweepResult :type Hit%20Result%20Structure%20%28by%20ref%29))
  (Audio|Components|Audio|Stop (stale EventBeginPlay _returnvalue))
  (bind _returnvalue (Audio|SpawnSound2D "/Game/Sound/Battle.Battle" 1.0 1.0 0.0 0))
  (Variables|Default|SetBattleMusic _returnvalue)
  (Collision|SetCollisionEnabled (Variables|Default|GetBox) "NoCollision")
  (bind _outactors (Actor|GetAllActorsOfClass "/Script/ClairObscur.PlayerBase"))
  (for _array_element _outactors
    (Class|PlayerFSM|EnterCombatMode (Variables|/Script/ClairObscur.PlayerBase|Getfsm _array_element)))
  (bind _outactors_2 (Actor|GetAllActorsOfClass "/Game/Game/BattleSystem/BP_BattleManager.BP_BattleManager_C"))
  (bind _output_get (Variables|Default|SetBM (Utilities|Array|Get(acopy) _outactors_2)))
  (Utilities|IsValid _output_get
    (:Is%20Valid
      (Class|BattleManager|StartBattle (Variables|Default|GetBm))
      (bind _outactors_3 (Actor|GetAllActorsOfClass "/Game/Enemy/BP_Enemy.BP_Enemy_C"))
      (Transformation|SetActorScale3D (Utilities|Array|Get(acopy) _outactors_3) "2.000000,2.000000,2.000000")
      (Components|Animation|SetAnimationMode (Variables|/Script/Engine.Character|GetMesh (Utilities|Array|Get(acopy) _outactors_3)) "AnimationBlueprint" true)
      (Components|SkeletalMesh|SetAnimInstanceClass (Variables|/Script/Engine.Character|GetMesh (Utilities|Array|Get(acopy) _outactors_3)) "/Game/Enemy/ABP_Enemy.ABP_Enemy_C")
      (Class|Enemy|ReinitializeAnimInstance (Utilities|Array|Get(acopy) _outactors_3))
      (Game|Player|SetViewTargetwithBlend (Game|GetPlayerController 0) (Variables|Default|GetBM) 1.0 "VTBlend_EaseInOut" 0.0 false))))

(event Custom|LevelsequenceEnd
  (bind _outactors (Actor|GetAllActorsOfClass "/Script/ClairObscur.PlayerBase"))
  (for _array_element _outactors
    (Class|PlayerFSM|EnterCombatMode (Variables|/Script/ClairObscur.PlayerBase|Getfsm _array_element)))
  (bind _outactors_2 (Actor|GetAllActorsOfClass "/Game/Game/BattleSystem/BP_BattleManager.BP_BattleManager_C"))
  (bind _output_get (Variables|Default|SetBM (Utilities|Array|Get(acopy) _outactors_2)))
  (Utilities|IsValid _output_get
    (:Is%20Valid
      (Class|BattleManager|StartBattle (Variables|Default|GetBm))
      (bind _outactors_3 (Actor|GetAllActorsOfClass "/Game/Enemy/BP_Enemy.BP_Enemy_C"))
      (Transformation|SetActorScale3D (Utilities|Array|Get(acopy) _outactors_3) "2.000000,2.000000,2.000000")
      (Components|Animation|SetAnimationMode (Variables|/Script/Engine.Character|GetMesh (Utilities|Array|Get(acopy) _outactors_3)) "AnimationBlueprint" true)
      (Components|SkeletalMesh|SetAnimInstanceClass (Variables|/Script/Engine.Character|GetMesh (Utilities|Array|Get(acopy) _outactors_3)) "/Game/Enemy/ABP_Enemy.ABP_Enemy_C")
      (Class|Enemy|ReinitializeAnimInstance (Utilities|Array|Get(acopy) _outactors_3))
      (Game|Player|SetViewTargetwithBlend (Game|GetPlayerController 0) (Variables|Default|GetBM) 1.0 "VTBlend_EaseInOut" 0.0 false))))

(event Collision|EventActorBeginOverlap
  (params (OtherActor :type Actor%20Object%20Reference)))

(event EventTick
  (params (DeltaSeconds :type Float%20%28single-precision%29)))

(event EventBeginPlay
  (bind _returnvalue (Audio|SpawnSound2D "/Game/Sound/Explore.Explore" 1.0 1.0 0.0 0)))

(fn ConstructionScript)