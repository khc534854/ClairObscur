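; BP_TestBattleManager is a test battle manager that prototypes timed skill input between a player party and an enemy party.
; On BeginPlay it gathers BP_TestPlayer and BP_TestEnemy actors, adds a timing widget and enables input.
; Q or E starts the widget's timing action, then after a delay plays the first player's or enemy's first skill montage.
; Space checks the timing window, prints a good or bad result and resets the widget.
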(event EventBeginPlay
  (bind _outactors (Actor|GetAllActorsOfClass "/Game/Game/BattleSystem/BP_TestPlayer.BP_TestPlayer_C"))
  (Variables|Default|SetPlayerParty _outactors)
  (bind _outactors_2 (Actor|GetAllActorsOfClass "/Game/Game/BattleSystem/BP_TestEnemy.BP_TestEnemy_C"))
  (Variables|Default|SetEnemyParty _outactors_2)
  (bind _returnvalue (UserInterface|CreateWidget "/Game/Game/BattleSystem/TestUI/WBP_TESTTiming.WBP_TESTTiming_C"))
  (bind _output_get (Variables|Default|SetTimingWidget _returnvalue))
  (UserInterface|Viewport|AddtoViewport _output_get 0)
  (Input|EnableInput (Game|GetPlayerController 0)))

(event Input|KeyboardEvents|E
  (params (Key :type Key%20Structure))
  (bind _enemyparty (Variables|Default|GetEnemyParty))
  (bind _output (Utilities|Array|Get(acopy) _enemyparty))
  (:Released
    (Default|TimingAction (Variables|Default|GetTimingWidget))
    (Utilities|FlowControl|Delay 2.0)
    (Components|Animation|PlayAnimation (Variables|/Script/Engine.Character|GetMesh _output) (Variables|/Script/ClairObscur.SkillDataAsset|GetSkillMontage (Utilities|Array|Get(acopy) (Variables|/Game/Game/BattleSystem/BP_TestEnemy.BP_TestEnemy_C|GetSkillList _output))) false)))

(event Input|KeyboardEvents|SpaceBar
  (params (Key :type Key%20Structure))
  (bind _timingwidget (Variables|Default|GetTimingWidget))
  (bind _timingtime (Variables|/Game/Game/BattleSystem/TestUI/WBP_TESTTiming.WBP_TESTTiming_C|GetTimingTime _timingwidget))
  (:Pressed
    (if (Variables|/Game/Game/BattleSystem/TestUI/WBP_TESTTiming.WBP_TESTTiming_C|GetbIsTiming _timingwidget)
      (if (and (< _timingtime 2.0) (> _timingtime 1.5))
        (Development|PrintString "Good Timing!")
        (else
          (Development|PrintString "Bad Timing..")))
      (Default|Reset _timingwidget))))

(event Input|KeyboardEvents|Q
  (params (Key :type Key%20Structure))
  (bind _playerparty (Variables|Default|GetPlayerParty))
  (bind _output (Utilities|Array|Get(acopy) _playerparty))
  (:Released
    (Default|TimingAction (Variables|Default|GetTimingWidget))
    (Utilities|FlowControl|Delay 2.0)
    (Components|Animation|PlayAnimation (Variables|/Script/Engine.Character|GetMesh _output) (Variables|/Script/ClairObscur.SkillDataAsset|GetSkillMontage (Utilities|Array|Get(acopy) (Variables|/Game/Game/BattleSystem/BP_TestPlayer.BP_TestPlayer_C|GetSkillList _output))) false)))

(fn ConstructionScript)